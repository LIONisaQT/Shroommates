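; Mama Mush NPC that delivers story dialog for the room she occupies.
; Teleport moves her to fixed bathroom, living room, kitchen or attic spots, starting in the bathroom and disabling her talk trigger in the attic.
; Player overlap disables jumping, enables tick and fills TextArray with voiced, multi-speaker lines.
; Lines branch on BP_Merchant's rescue flags, and the first post-baby-rescue conversation sets PostBabySaved so it changes afterward.
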(event `InputAction|Interact` :consume false
  (params (Key :type "Key Structure"))
  ;[1 0.2292 0.9547] Overload Interact (open shop)
  (:`Pressed`
    (`KismetSystemLibrary.PrintString` "")))

(event `self.ReceiveBeginPlay`
  ;[0.3674 1 0.8182] Overload BeginPlay
  (`|ExecutionSequence`
    (:`then_0`
      ;;[0 1 0.3042] Create widgets
      (`/Engine/EditorBlueprintResources/StandardMacros.IsValid` (`self.dialogWidget`)
        (:`Is Not Valid`
          (bind _returnvalue (`|CreateWidget` "/Game/Dialog/WB_Dialog.WB_Dialog_C"))
          (set `self.dialogWidget` _returnvalue))))
    (:`then_1`
      ;;[1 1 1] Set player reference to avoid multiple casts
      (bind _asshroommate_proto_character (cast `ShroommateProtoCharacter` (`GameplayStatics.GetPlayerCharacter` 0)))
      (set `self.playerRef` _asshroommate_proto_character))
    (:`then_2`
      ;;[0.1162 0.4479 0.05799] Guarentee Mama Mush is in the bathroom in the beginning
      (`self.Teleport` "NewEnumerator1"))
    (:`then_3`
      ;;[0.526 0.526 0.526] Hide text
      (`SceneComponent.SetVisibility` (`self.TextRender`) false false))))

(event `self.TextTrigger.OnComponentBeginOverlap`
  (params (OverlappedComponent :type "PrimitiveComponent Object Reference") (OtherActor :type "Actor Object Reference") (OtherComp :type "PrimitiveComponent Object Reference") (OtherBodyIndex :type Integer) (bFromSweep :type Boolean) (SweepResult :type "HitResult Structure (by ref)"))
  (bind _playerref (`self.playerRef`))
  ;[1 1 1] Overload BeginOverlap
  (if (== OtherActor _playerref)
    (`|ExecutionSequence`
      (:`then_0`
        (`self.DisableJump` _playerref)
        (set `ShroommateProtoCharacter.TalkMamaCheck` true (`self.playerRef`))
        (`self.SetActorTickEnabled` true))
      (:`then_1`
        (`self.SetTextByRoom` (`self.currentRoom`))))))

(event `self.Teleport`
  (params (location :type "/Game/Dialog/E_CurrentRoom Enum" :default "NewEnumerator0"))
  ;[0.5714 0.2865 1] Overload teleport
  ;;[0.2448 0.499 1] Bathroom
  (if (`|EnumEquality` location "NewEnumerator1")
    (`self.K2_TeleportTo` (-14329.0 -24421.0 182.279236) (struct :`Yaw` -90.0))
    (set `self.currentRoom` "NewEnumerator1")
    (`PrimitiveComponent.SetCollisionEnabled` (`self.TextTrigger`) "QueryOnly")
    (else
      ;;[1 0.5362 0.09896] Living room
      (if (`|EnumEquality` location "NewEnumerator2")
        (`self.K2_TeleportTo` (-14014.0 -22974.0 182.24054) (struct :`Yaw` -160.0))
        (set `self.currentRoom` "NewEnumerator2")
        (`PrimitiveComponent.SetCollisionEnabled` (`self.TextTrigger`) "QueryOnly")
        (else
          ;;[1 0.07292 0.07292] Kitchen
          (if (`|EnumEquality` location "NewEnumerator3")
            (`self.K2_TeleportTo` (-12121.0 -23706.0 78.0) (struct :`Yaw` 90.0))
            (set `self.currentRoom` "NewEnumerator3")
            (`PrimitiveComponent.SetCollisionEnabled` (`self.TextTrigger`) "QueryOnly")
            (else
              ;;[1 1 1] Attic
              (if (`|EnumEquality` location "NewEnumerator5")
                (`self.K2_TeleportTo` (-12823.0 -24493.0 392.0) (struct :`Yaw` -40.000061))
                (set `self.currentRoom` "NewEnumerator5")
                (`PrimitiveComponent.SetCollisionEnabled` (`self.TextTrigger`) "NoCollision")))))))))

(event `self.SetTextByRoom`
  (params (NewParam :type "/Game/Dialog/E_CurrentRoom Enum" :default "NewEnumerator0"))
  (bind _textarray (`self.textArray`))
  (bind _textarray_2 (`self.textArray`))
  ;[1 0.9635 0.2865] Overload SetTextByRoom
  (`|ExecutionSequence`
    (:`then_0`
      ;;[0.09375 0.3479 1] Make sure array is empty before adding new text
      (`KismetArrayLibrary.Array_Clear` (`self.textArray`)))
    (:`then_1`
      ;;[0.151 0.8913 1] Bathroom
      (if (`|EnumEquality` NewParam "NewEnumerator1")
        (`KismetArrayLibrary.Array_Add` (`self.textArray`) (make `/Game/Dialog/S_Dialog` "Let's get out of here and find Baby Mush!" "Mama Mush" "/Game/Sounds/Voices/MamaMush/VA_LetsFindBaby.VA_LetsFindBaby"))
        (else
          ;;[1 0.4162 0.2188] Living Room
          (if (`|EnumEquality` NewParam "NewEnumerator2")
            (bind _outactors (`GameplayStatics.GetAllActorsOfClass` "/Game/Dialog/BP_Merchant.BP_Merchant_C"))
            (bind _output (`|GetArrayItem` _outactors))
            (if (`/Game/Dialog/BP_Merchant.babySaved` _output)
              (if (`/Game/Dialog/BP_Merchant.postBabySaved` _output)
                (`KismetArrayLibrary.Array_Add` _textarray_2 (make `/Game/Dialog/S_Dialog` "I hope grandpa’s okay. I know he can’t walk very well without his cane..." "Mama Mush" "/Game/Sounds/Voices/MamaMush/VA_HopeGrandpaOkay.VA_HopeGrandpaOkay"))
                (`KismetArrayLibrary.Array_Add` _textarray_2 (make `/Game/Dialog/S_Dialog` "Chop! Chop! Fwah!!!! Fwah!!!! Fiyah!!!!" "Baby Mush" "/Game/Sounds/Voices/BabyMush/VA_BabyNoises.VA_BabyNoises"))
                (else
                  (`KismetArrayLibrary.Array_Add` _textarray_2 (make `/Game/Dialog/S_Dialog` "So ya found the kid!" "Merchant" "/Game/Sounds/Voices/Merchant/VA_FoundTheKid.VA_FoundTheKid"))
                  (`KismetArrayLibrary.Array_Add` _textarray_2 (make `/Game/Dialog/S_Dialog` "Gwandpa..." "Baby Mush" "/Game/Sounds/Voices/BabyMush/VA_Gwandpa01.VA_Gwandpa01"))
                  (`KismetArrayLibrary.Array_Add` _textarray_2 (make `/Game/Dialog/S_Dialog` "You saw Grandpa?! Where did he go?" "Mama Mush" "/Game/Sounds/Voices/MamaMush/VA_SawGrandpa.VA_SawGrandpa"))
                  (`KismetArrayLibrary.Array_Add` _textarray_2 (make `/Game/Dialog/S_Dialog` "Chop! Chop! Fwah!!!! Fwah!!!! Fiyah!!!!" "Baby Mush" "/Game/Sounds/Voices/BabyMush/VA_BabyNoises.VA_BabyNoises"))
                  (`KismetArrayLibrary.Array_Add` _textarray_2 (make `/Game/Dialog/S_Dialog` "Ooooh…..sounds like Grandpa’s gonna be made into a fine shiitake stir fry. Might wanna get to the kitchen before it’s too late." "Merchant" "/Game/Sounds/Voices/Merchant/VA_Shiitake.VA_Shiitake"))
                  (`KismetArrayLibrary.Array_Add` _textarray_2 (make `/Game/Dialog/S_Dialog` "But how? How do we get to him?" "Mama Mush" "/Game/Sounds/Voices/MamaMush/VA_ButHow.VA_ButHow"))
                  (`KismetArrayLibrary.Array_Add` _textarray_2 (make `/Game/Dialog/S_Dialog` "There's a key somewhere by the couch I bet." "Merchant" "/Game/Sounds/Voices/Merchant/VA_TheresAKey.VA_TheresAKey"))
                  (`KismetArrayLibrary.Array_Add` _textarray_2 (make `/Game/Dialog/S_Dialog` "She’s really invested in that game... bet she wouldn’t even notice if you ran right in front of her! We’re gonna need some other kind of distraction…" "Merchant" "/Game/Sounds/Voices/Merchant/VA_InvestedInGame.VA_InvestedInGame"))
                  (set `/Game/Dialog/BP_Merchant.postBabySaved` true _output)))
              (else
                (`KismetArrayLibrary.Array_Add` _textarray_2 (make `/Game/Dialog/S_Dialog` "Save my baby!" "Mama Mush" "/Game/Sounds/Voices/MamaMush/VA_Hmm.VA_Hmm"))))
            (else
              ;;[1 0.09375 0.09375] Kitchen
              (if (`|EnumEquality` NewParam "NewEnumerator3")
                (bind _outactors_2 (`GameplayStatics.GetAllActorsOfClass` "/Game/Dialog/BP_Merchant.BP_Merchant_C"))
                (if (`/Game/Dialog/BP_Merchant.grandpaSaved` (`|GetArrayItem` _outactors_2))
                  (`KismetArrayLibrary.Array_Add` _textarray (make `/Game/Dialog/S_Dialog` "Thanks, sonny! Oh, I could really go for some good old stew right now." "Grandpa Mush" "/Game/Sounds/Voices/GrandpaMush/VA_Stew.VA_Stew"))
                  (`KismetArrayLibrary.Array_Add` _textarray (make `/Game/Dialog/S_Dialog` "Gwandpa! Gwandpa! Chop! Chop!" "Baby Mush" "/Game/Sounds/Voices/BabyMush/VA_GwandpaChop.VA_GwandpaChop"))
                  (`KismetArrayLibrary.Array_Add` _textarray (make `/Game/Dialog/S_Dialog` "Oh, thank goodness! Let's get home before Grandpa starts complaining." "Mama Mush" "/Game/Sounds/Voices/MamaMush/VA_GrandpaComplain.VA_GrandpaComplain"))
                  (else
                    (`KismetArrayLibrary.Array_Add` _textarray (make `/Game/Dialog/S_Dialog` "I hope grandpa's okay, I know he can't walk very well without his cane." "Mama Mush" "/Game/Sounds/Voices/MamaMush/VA_HopeGrandpaOkay.VA_HopeGrandpaOkay"))
                    (`KismetArrayLibrary.Array_Add` _textarray (make `/Game/Dialog/S_Dialog` "Gwandpa..." "Baby Mush" "/Game/Sounds/Voices/BabyMush/VA_Gwandpa02.VA_Gwandpa02"))))))))))))

(fn `UserConstructionScript`)
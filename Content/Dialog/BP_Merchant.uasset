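; Merchant rat NPC that teleports between rooms, giving voiced story dialog, a living-room store and the game's ending.
; Entering its trigger disables jump, enables camera-facing text, swaps carried Baby or Grandpa for placed items, and rebuilds the line array from room and rescue flags.
; Jump steps through lines with portraits, movement locked and HUD hidden; Interact toggles the store.
; After the attic dialog, Jump advances ending slides into credits.
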(event `self.ReceiveBeginPlay`
  (`|ExecutionSequence`
    (:`then_0`
      ;[0 1 0.3042] Create widgets
      (`|ExecutionSequence`
        (:`then_0`
          (`/Engine/EditorBlueprintResources/StandardMacros.IsValid` (`self.dialogWidget`)
            (:`Is Not Valid`
              (bind _returnvalue (`|CreateWidget` "/Game/Dialog/WB_Dialog.WB_Dialog_C"))
              (set `self.dialogWidget` _returnvalue))))
        (:`then_1`
          (`/Engine/EditorBlueprintResources/StandardMacros.IsValid` (`self.storeWidget`)
            (:`Is Not Valid`
              (bind _returnvalue_2 (`|CreateWidget` "/Game/UI/SkillTree/UI_store.UI_store_C"))
              (set `self.storeWidget` _returnvalue_2))))
        (:`then_2`
          (`/Engine/EditorBlueprintResources/StandardMacros.IsValid` (`self.endingWidget`)
            (:`Is Not Valid`
              (bind _returnvalue_3 (`|CreateWidget` "/Game/Dialog/WB_Endings.WB_Endings_C"))
              (set `self.endingWidget` _returnvalue_3))))))
    (:`then_1`
      ;[1 1 1] Set player reference to avoid multiple casts
      (bind _asshroommate_proto_character (cast `ShroommateProtoCharacter` (`GameplayStatics.GetPlayerCharacter` 0)))
      (set `self.playerRef` _asshroommate_proto_character))
    (:`then_2`
      ;[0.1162 0.4479 0.05799] Guarentee merchant is in the garden in the beginning
      (`self.Teleport` "NewEnumerator0"))
    (:`then_3`
      ;[0.526 0.526 0.526] Hide text
      (`SceneComponent.SetVisibility` (`self.TextRender`) false false))))

(event `self.TextTrigger.OnComponentBeginOverlap`
  (params (OverlappedComponent :type "PrimitiveComponent Object Reference") (OtherActor :type "Actor Object Reference") (OtherComp :type "PrimitiveComponent Object Reference") (OtherBodyIndex :type Integer) (bFromSweep :type Boolean) (SweepResult :type "HitResult Structure (by ref)"))
  (bind _currentroom (`self.currentRoom`))
  (bind _playerref (`self.playerRef`))
  (bind _output (`|GetArrayItem` (`self.GetAttachedActors` _playerref)))
  (bind _output_2 (`|GetArrayItem` (`self.GetAttachedActors` _playerref)))
  ;[0.3073 1 0.5329] Collision with text trigger
  (if (== OtherActor _playerref)
    (`|ExecutionSequence`
      (:`then_0`
        (`self.DisableJump` _playerref)
        (set `ShroommateProtoCharacter.TalkRatCheck` true (`self.playerRef`))
        (`self.SetActorTickEnabled` true))
      (:`then_1`
        ;;[1 0.6314 0.3385] Living room logic
        (if (`|EnumEquality` _currentroom "NewEnumerator2")
          ;;;[0.3229 0.9074 1] Put baby down (this was the best solution as detach wouldn't correctly set location)
          (if (== (`KismetSystemLibrary.GetObjectName` _output) "BP_Item_BabyMush_2")
            (`self.K2_DestroyActor` _output)
            (bind _returnvalue (`|SpawnActorFromClass` "/Game/Blueprints/GameObjects/PickUp/BP_Item_BabyMush.BP_Item_BabyMush_C" (`KismetMathLibrary.MakeTransform` (-14025.0 -22983.0 176.0) (struct :`Yaw` 180.0)) "Undefined" "OverrideRootScale" null null))
            (`GameplayStatics.PlaySoundAtLocation` "/Game/Sounds/Voices/BabyMush/VA_Babble04.VA_Babble04" (`self.K2_GetActorLocation` _returnvalue))
            (set `self.babySaved` true)
            (bind _asbp_skill_tree_controller (cast `/Game/Blueprints/BP_SkillTreeController` (`GameplayStatics.GetPlayerController` 0)))
            (set `SkillTreeController.haskitchenitem` false _asbp_skill_tree_controller)
            (bind _returnvalue_2 (`|SpawnActorFromClass` "/Game/Blueprints/GameObjects/PickUp/BP_Item_Key.BP_Item_Key_C" (`KismetMathLibrary.MakeTransform` (-13760.0 -23390.0 140.0) (struct :`Yaw` 180.0) (0.3 0.3 0.3)) "Undefined" "OverrideRootScale" null null))
            (set `AudioComponent.AttenuationSettings` "/Game/Sounds/SoundEffects/Key/SA_Key02.SA_Key02" (`/Game/Blueprints/GameObjects/PickUp/BP_Item_Key.Audio` _returnvalue_2)))
          (else
            ;;[1 0.1667 0.1667] Kitchen logic
            (if (`|EnumEquality` _currentroom "NewEnumerator3")
              (if (== (`KismetSystemLibrary.GetDisplayName` _output_2) "OldMush-Idle_Blueprint")
                (`self.K2_DestroyActor` _output_2)
                (bind _returnvalue_3 (`|SpawnActorFromClass` "/Game/Blueprints/GameObjects/PickUp/BP_Item_Grandpa.BP_Item_Grandpa_C" (`KismetMathLibrary.MakeTransform` (-12142.0 -23728.0 93.804077) (struct :`Yaw` 9.999969)) "Undefined" "OverrideRootScale" null null))
                (bind _skeletalmeshcomponent (`SkeletalMeshActor.SkeletalMeshComponent` _returnvalue_3))
                (`SkeletalMeshComponent.SetAnimation` _skeletalmeshcomponent "/Game/MushFam/OldMush-Idle_Anim.OldMush-Idle_Anim")
                (`SkeletalMeshComponent.Play` _skeletalmeshcomponent true)
                (set `self.grandpaSaved` true)
                (bind _asshroommate_proto_character (cast `ShroommateProtoCharacter` (`GameplayStatics.GetPlayerCharacter` 0)))
                (set `ShroommateProtoCharacter.KitchenLevelCheck` true _asshroommate_proto_character)
                (bind _asbp_skill_tree_controller_2 (cast `/Game/Blueprints/BP_SkillTreeController` (`GameplayStatics.GetPlayerController` 0)))
                (set `SkillTreeController.haskitchenitem` false _asbp_skill_tree_controller_2))))))
      (:`then_2`
        (`self.SetTextByRoom` _currentroom)))))

(event `InputAction|Interact` :consume false
  (params (Key :type "Key Structure"))
  ;[0.5987 0.3177 1] Open store
  (:`Pressed`
    (if (and (`PrimitiveComponent.IsOverlappingActor` (`self.TextTrigger`) (`self.playerRef`)) (`|EnumEquality` (`self.currentRoom`) "NewEnumerator2"))
      (if (`self.opened`)
        _
        (elif (`self.storeOpened`)
          (`self.CloseStore`)
          (else
            (`self.OpenStore`)))))))

(event `self.ReceiveTick`
  (params (DeltaSeconds :type "Float (single-precision)"))
  ;[1 0.3714 0.25] Only runs when player is inside trigger box
  (`self.LookAtCamera`))

(event `InputAction|Jump` :consume false
  (params (Key :type "Key Structure"))
  (bind _audio (`self.Audio`))
  (bind _audio_2 (`self.Audio`))
  (bind _audio_3 (`self.Audio`))
  (bind _audio_4 (`self.Audio`))
  (bind _audio_5 (`self.Audio`))
  (bind _audio_6 (`self.Audio`))
  (bind _endingwidget (`self.endingWidget`))
  (bind _endingcounter (`self.endingCounter`))
  (bind _textarray (`self.textArray`))
  (bind _currtext (`self.currText`))
  (bind (_output_text _output_source _output_voice) (break `/Game/Dialog/S_Dialog` (`|GetArrayItem` _textarray _currtext)))
  (bind _background (`/Game/Dialog/WB_Endings.Background` _endingwidget))
  (bind _brush_imagesize (break `SlateBrush` (`Image.Brush` _background)))
  ;[0 0.4429 1] Open dialog
  (:`Pressed`
    (if (`PrimitiveComponent.IsOverlappingActor` (`self.TextTrigger`) (`self.playerRef`))
      (if (`self.storeOpened`)
        _
        (elif (== _currtext (`KismetArrayLibrary.Array_Length` _textarray))
          (`AudioComponent.Stop` (`self.Audio`))
          (`self.CloseDialog`)
          (if (`self.gameEnd`)
            (if (< (`self.endingCounter`) 10)
              (`|ExecutionSequence`
                (:`then_0`
                  (`UserWidget.AddToViewport` _endingwidget 0))
                (:`then_1`
                  (if (== _endingcounter 0)
                    (`Image.SetBrush` _background (make `SlateBrush` _brush_imagesize (struct) (struct :`SpecifiedColor` (struct :`R` 1.0 :`G` 1.0 :`B` 1.0 :`A` 1.0) :`ColorUseRule` "UseColor_Specified") "/Game/Textures/Endings/1_fight.1_fight"))
                    (`/Engine/EditorBlueprintResources/StandardMacros.IncrementInt` (`self.endingCounter`))
                    (elif (== _endingcounter 1)
                      (`Image.SetBrush` _background (make `SlateBrush` _brush_imagesize (struct) (struct :`SpecifiedColor` (struct :`R` 1.0 :`G` 1.0 :`B` 1.0 :`A` 1.0) :`ColorUseRule` "UseColor_Specified") "/Game/Textures/Endings/2_fight.2_fight"))
                      (`/Engine/EditorBlueprintResources/StandardMacros.IncrementInt` (`self.endingCounter`))
                      (elif (== _endingcounter 2)
                        (`Image.SetBrush` _background (make `SlateBrush` _brush_imagesize (struct) (struct :`SpecifiedColor` (struct :`R` 1.0 :`G` 1.0 :`B` 1.0 :`A` 1.0) :`ColorUseRule` "UseColor_Specified") "/Game/Textures/Endings/3_dialogue.3_dialogue"))
                        (`/Engine/EditorBlueprintResources/StandardMacros.IncrementInt` (`self.endingCounter`)
                          (:`  `
                            (`AudioComponent.SetSound` _audio_2 "/Game/Sounds/Voices/Merchant/VA_YouGotMe.VA_YouGotMe")
                            (`AudioComponent.Play` _audio_2 0.0)))
                        (elif (== _endingcounter 3)
                          (`Image.SetBrush` _background (make `SlateBrush` _brush_imagesize (struct) (struct :`SpecifiedColor` (struct :`R` 1.0 :`G` 1.0 :`B` 1.0 :`A` 1.0) :`ColorUseRule` "UseColor_Specified") "/Game/Textures/Endings/4_dialogue.4_dialogue"))
                          (`/Engine/EditorBlueprintResources/StandardMacros.IncrementInt` (`self.endingCounter`)
                            (:`  `
                              (`AudioComponent.SetSound` _audio_3 "/Game/Sounds/Voices/Merchant/VA_PackAPunch.VA_PackAPunch")
                              (`AudioComponent.Play` _audio_3 0.0)))
                          (elif (== _endingcounter 4)
                            (`Image.SetBrush` _background (make `SlateBrush` _brush_imagesize (struct) (struct :`SpecifiedColor` (struct :`R` 1.0 :`G` 1.0 :`B` 1.0 :`A` 1.0) :`ColorUseRule` "UseColor_Specified") "/Game/Textures/Endings/5_dialogue.5_dialogue"))
                            (`/Engine/EditorBlueprintResources/StandardMacros.IncrementInt` (`self.endingCounter`)
                              (:`  `
                                (`AudioComponent.SetSound` _audio_4 "/Game/Sounds/Voices/Merchant/VA_Huh.VA_Huh")
                                (`AudioComponent.Play` _audio_4 0.0)))
                            (elif (== _endingcounter 5)
                              (`Image.SetBrush` _background (make `SlateBrush` _brush_imagesize (struct) (struct :`SpecifiedColor` (struct :`R` 1.0 :`G` 1.0 :`B` 1.0 :`A` 1.0) :`ColorUseRule` "UseColor_Specified") "/Game/Textures/Endings/6_dialogue.6_dialogue"))
                              (`/Engine/EditorBlueprintResources/StandardMacros.IncrementInt` (`self.endingCounter`)
                                (:`  `
                                  (`AudioComponent.SetSound` _audio_5 "/Game/Sounds/Voices/Merchant/VA_YouWantStay.VA_YouWantStay")
                                  (`AudioComponent.Play` _audio_5 0.0)))
                              (elif (== _endingcounter 6)
                                (`Image.SetBrush` _background (make `SlateBrush` _brush_imagesize (struct) (struct :`SpecifiedColor` (struct :`R` 1.0 :`G` 1.0 :`B` 1.0 :`A` 1.0) :`ColorUseRule` "UseColor_Specified") "/Game/Textures/Endings/7_dialogue.7_dialogue"))
                                (`/Engine/EditorBlueprintResources/StandardMacros.IncrementInt` (`self.endingCounter`)
                                  (:`  `
                                    (`AudioComponent.SetSound` _audio_6 "/Game/Sounds/Voices/Merchant/VA_EvenAfterEverything.VA_EvenAfterEverything")
                                    (`AudioComponent.Play` _audio_6 0.0)))
                                (elif (== _endingcounter 7)
                                  (`Image.SetBrush` _background (make `SlateBrush` _brush_imagesize (struct) (struct :`SpecifiedColor` (struct :`R` 1.0 :`G` 1.0 :`B` 1.0 :`A` 1.0) :`ColorUseRule` "UseColor_Specified") "/Game/Textures/Endings/8_dialogue.8_dialogue"))
                                  (`/Engine/EditorBlueprintResources/StandardMacros.IncrementInt` (`self.endingCounter`)
                                    (:`  `
                                      (`AudioComponent.SetSound` _audio "/Game/Sounds/Voices/Merchant/VA_ThankYou.VA_ThankYou")
                                      (`AudioComponent.Play` _audio 0.0)))
                                  (elif (== _endingcounter 8)
                                    (`Image.SetBrush` _background (make `SlateBrush` _brush_imagesize (struct) (struct :`SpecifiedColor` (struct :`R` 1.0 :`G` 1.0 :`B` 1.0 :`A` 1.0) :`ColorUseRule` "UseColor_Specified") "/Game/Textures/Endings/9_end.9_end"))
                                    (`/Engine/EditorBlueprintResources/StandardMacros.IncrementInt` (`self.endingCounter`))
                                    (elif (== _endingcounter 9)
                                      (`Widget.RemoveFromParent` _background)
                                      (bind _returnvalue (`|CreateWidget` "/Game/Dialog/Credz.Credz_C"))
                                      (`UserWidget.AddToViewport` _returnvalue 0)
                                      (set `self.credits` true))))))))))))))
            (else
              (set `self.currText` 0)))
          (else
            (`self.OpenDialog` _output_text _output_source _output_voice)
            (`/Engine/EditorBlueprintResources/StandardMacros.IncrementInt` (`self.currText`))))))))

(event `self.TextTrigger.OnComponentEndOverlap`
  (params (OverlappedComponent :type "PrimitiveComponent Object Reference") (OtherActor :type "Actor Object Reference") (OtherComp :type "PrimitiveComponent Object Reference") (OtherBodyIndex :type Integer))
  (bind _playerref (`self.playerRef`))
  ;[1 0.1823 0.197] Leave text trigger
  (if (== OtherActor _playerref)
    (`self.EnableJump` _playerref)
    (set `ShroommateProtoCharacter.TalkRatCheck` false _playerref)
    (set `ShroommateProtoCharacter.TalkMamaCheck` false _playerref)
    (`self.SetActorTickEnabled` false)))

(fn `CloseDialog`
  (`|ExecutionSequence`
    (:`then_0`
      (`Widget.RemoveFromParent` (`self.dialogWidget`)))
    (:`then_1`
      (`Controller.ResetIgnoreMoveInput` (`GameplayStatics.GetPlayerController` 0)))
    (:`then_2`
      (`GameplayStatics.PlaySound2D` (`self.closeSound`)))
    (:`then_3`
      (set `self.opened` false))
    (:`then_4`
      (bind _foundwidgets (`WidgetBlueprintLibrary.GetAllWidgetsOfClass` "/Game/UI/BP_GameHUD.BP_GameHUD_C"))
      (for _array_element _foundwidgets
        (`Widget.SetVisibility` _array_element "Visible")))))

(fn `CloseStore`
  (`|ExecutionSequence`
    (:`then_0`
      (`Widget.RemoveFromParent` (`self.storeWidget`)))
    (:`then_1`
      (`Controller.ResetIgnoreMoveInput` (`GameplayStatics.GetPlayerController` 0)))
    (:`then_2`
      (set `self.storeOpened` false))))

(fn `DisableJump`
  (params (Player :type "ShroommateProtoCharacter Object Reference"))
  (set `ShroommateProtoCharacter.jumpEnabled` false Player))

(fn `EnableJump`
  (params (Player :type "ShroommateProtoCharacter Object Reference"))
  (set `ShroommateProtoCharacter.jumpEnabled` true Player))

(fn `LookAtCamera`
  (bind _textrender (`self.TextRender`))
  (bind (_returnvalue_roll _returnvalue_pitch _returnvalue_yaw) (`KismetMathLibrary.BreakRotator` (`KismetMathLibrary.Conv_VectorToRotator` (`KismetMathLibrary.GetDirectionUnitVector` (`SceneComponent.K2_GetComponentLocation` (`PlayerCameraManager.TransformComponent` (`GameplayStatics.GetPlayerCameraManager` 0))) (`SceneComponent.K2_GetComponentLocation` _textrender)))))
  (bind _result (`/Engine/EditorBlueprintResources/StandardMacros.NegateFloat` _returnvalue_pitch)
    (:`  `
      (`SceneComponent.K2_SetWorldRotation` _textrender (`KismetMathLibrary.MakeRotator` 0.0 _result (+ _returnvalue_yaw 180.0)) false false))))

(fn `OpenDialog`
  (params (Text :type Text) (Source :type Text) (Voice :type "SoundWave Object Reference"))
  (locals (Merchant :type Text :default "NSLOCTEXT(\"\", \"296D11C948A13C2DBBF1FFA9A908C977\", \"Merchant\")") (MamaMush :type Text :default "NSLOCTEXT(\"\", \"082441FC4E1F9A36693B08A1038414F7\", \"Mama Mush\")") (BabyMush :type Text :default "NSLOCTEXT(\"\", \"2BF6262146C4A132B648E2BCEB0F895E\", \"Baby Mush\")") (GrandpaMush :type Text :default "NSLOCTEXT(\"\", \"40173E96465B48D9928929B913689A40\", \"Grandpa Mush\")") (Roommate2 :type Text :default "NSLOCTEXT(\"\", \"43F718D14A595DEEA7B45DAF3FD6BD83\", \"Roommate2\")"))
  (bind _audio (`self.Audio`))
  (bind _dialogwidget (`self.dialogWidget`))
  (bind _portrait (`/Game/Dialog/WB_Dialog.Portrait` _dialogwidget))
  (bind _brush_imagesize (break `SlateBrush` (`Image.Brush` _portrait)))
  (`|ExecutionSequence`
    (:`then_0`
      ;[1 0.1823 0.1823] Turn off player movement
      (`Controller.SetIgnoreMoveInput` (`GameplayStatics.GetPlayerController` 0) true))
    (:`then_1`
      ;[0.4792 0.4792 0.4792] Set dialog and put on screen and draw the correct portrait
      (`|ExecutionSequence`
        (:`then_0`
          (set `/Game/Dialog/WB_Dialog.dialog` Text _dialogwidget))
        (:`then_1`
          (bind _output_get (set `/Game/Dialog/WB_Dialog.speaker` Source _dialogwidget)))
        (:`then_2`
          (`UserWidget.AddToViewport` _dialogwidget 0))
        (:`then_3`
          (if (== _output_get (`local.Merchant`))
            (`Image.SetBrush` _portrait (make `SlateBrush` _brush_imagesize (struct) (struct :`SpecifiedColor` (struct :`R` 1.0 :`G` 1.0 :`B` 1.0 :`A` 1.0) :`ColorUseRule` "UseColor_Specified") "/Game/Textures/Portraits/T_Merchant_Portrait.T_Merchant_Portrait"))
            (elif (== _output_get (`local.MamaMush`))
              (`Image.SetBrush` _portrait (make `SlateBrush` _brush_imagesize (struct) (struct :`SpecifiedColor` (struct :`R` 1.0 :`G` 1.0 :`B` 1.0 :`A` 1.0) :`ColorUseRule` "UseColor_Specified") "/Game/Textures/Portraits/T_MamaMush_Portrait.T_MamaMush_Portrait"))
              (elif (== _output_get (`local.BabyMush`))
                (`Image.SetBrush` _portrait (make `SlateBrush` _brush_imagesize (struct) (struct :`SpecifiedColor` (struct :`R` 1.0 :`G` 1.0 :`B` 1.0 :`A` 1.0) :`ColorUseRule` "UseColor_Specified") "/Game/Textures/Portraits/T_BabyMush_Portrait.T_BabyMush_Portrait"))
                (elif (== _output_get (`local.GrandpaMush`))
                  (`Image.SetBrush` _portrait (make `SlateBrush` _brush_imagesize (struct) (struct :`SpecifiedColor` (struct :`R` 1.0 :`G` 1.0 :`B` 1.0 :`A` 1.0) :`ColorUseRule` "UseColor_Specified") "/Game/Textures/Portraits/T_GrandpaMush_Portrait.T_GrandpaMush_Portrait"))
                  (elif (`KismetTextLibrary.EqualEqual_TextText` _output_get (`local.Roommate2`))
                    (`Image.SetBrush` _portrait (make `SlateBrush` _brush_imagesize (struct) (struct :`SpecifiedColor` (struct :`R` 1.0 :`G` 1.0 :`B` 1.0 :`A` 1.0) :`ColorUseRule` "UseColor_Specified") "/Game/Textures/Portraits/T_Roommate02_Portrait.T_Roommate02_Portrait"))))))))))
    (:`then_2`
      ;[0.2708 0.8272 1] Play sound
      (`AudioComponent.SetSound` _audio Voice)
      (`AudioComponent.Play` _audio 0.0))
    (:`then_3`
      ;[0.5938 0.1206 0.1206] Deprecated
      (set `self.opened` true))
    (:`then_4`
      ;[0.1979 0.2472 1] Turn off HUD
      (bind _foundwidgets (`WidgetBlueprintLibrary.GetAllWidgetsOfClass` "/Game/UI/BP_GameHUD.BP_GameHUD_C"))
      (for _array_element _foundwidgets
        (`Widget.SetVisibility` _array_element "Hidden")))))

(fn `OpenStore`
  (bind _storewidget (`self.storeWidget`))
  (`|ExecutionSequence`
    (:`then_0`
      (`Controller.SetIgnoreMoveInput` (`GameplayStatics.GetPlayerController` 0) true))
    (:`then_1`
      ;[1 1 1] DIS is 4 CONTROLLER.
      (`UserWidget.AddToViewport` _storewidget 0)
      (`WidgetBlueprintLibrary.SetInputMode_UIOnlyEx` (`GameplayStatics.GetPlayerController` 0) (`/Game/UI/SkillTree/UI_store.lullaby` _storewidget)))
    (:`then_2`
      (set `self.storeOpened` true))
    (:`then_3`
      (`GameplayStatics.PlaySound2D` (`self.storeSound`)))))

(fn `SetText`
  (params (text :type Text) (source :type Text))
  (`|ExecutionSequence`
    (:`then_0`
      (set `self.Text` text))
    (:`then_1`
      (set `self.Source` source))))

(fn `SetTextByRoom`
  (params (NewParam :type "/Game/Dialog/E_CurrentRoom Enum" :default "NewEnumerator0"))
  (bind _textarray (`self.textArray`))
  (bind _textarray_2 (`self.textArray`))
  (bind _textarray_3 (`self.textArray`))
  (bind _textarray_4 (`self.textArray`))
  (`|ExecutionSequence`
    (:`then_0`
      ;[0.224 0.3611 1] Make sure array is empty before adding new text
      (`KismetArrayLibrary.Array_Clear` (`self.textArray`)))
    (:`then_1`
      ;[0.2838 1 0.2025] Garden
      (if (`|EnumEquality` NewParam "NewEnumerator0")
        (`KismetArrayLibrary.Array_Add` (`self.textArray`) (make `/Game/Dialog/S_Dialog` "You can always talk to me to get some advice and hear what I’m thinking. In fact, you should always try to listen to things I say! I also sell things! I’m a pretty useful rat, dontcha think?" "Merchant" "/Game/Sounds/Voices/Merchant/VA_CanAlwaysTalk.VA_CanAlwaysTalk"))
        (else
          ;[0.2552 0.7895 1] Bathroom
          (if (`|EnumEquality` NewParam "NewEnumerator1")
            (if (`ShroommateProtoCharacter.HasKey` (`self.playerRef`))
              (`KismetArrayLibrary.Array_Add` _textarray_3 (make `/Game/Dialog/S_Dialog` "Nice! Use the key on the door and show ourselves out." "Merchant" "/Game/Sounds/Voices/Merchant/VA_NiceUseKey.VA_NiceUseKey"))
              (else
                (`KismetArrayLibrary.Array_Add` _textarray_3 (make `/Game/Dialog/S_Dialog` "There’s a key somewhere in here I bet. If you listen, I think you can almost hear one…" "Merchant" "/Game/Sounds/Voices/Merchant/VA_TheresAKey.VA_TheresAKey"))))
            (else
              ;[0.6771 0.3941 0.1693] Living room
              (if (`|EnumEquality` NewParam "NewEnumerator2")
                (if (`self.babySaved`)
                  (if (`self.postBabySaved`)
                    (`KismetArrayLibrary.Array_Add` _textarray (make `/Game/Dialog/S_Dialog` "She’s really invested in that game... bet she wouldn’t even notice if you ran right in front of her! We’re gonna need some other kind of distraction…" "Merchant" "/Game/Sounds/Voices/Merchant/VA_InvestedInGame.VA_InvestedInGame"))
                    (else
                      (`KismetArrayLibrary.Array_Add` _textarray (make `/Game/Dialog/S_Dialog` "So ya found the kid!" "Merchant" "/Game/Sounds/Voices/Merchant/VA_FoundTheKid.VA_FoundTheKid"))
                      (`KismetArrayLibrary.Array_Add` _textarray (make `/Game/Dialog/S_Dialog` "Gwandpa..." "Baby Mush" "/Game/Sounds/Voices/BabyMush/VA_Gwandpa01.VA_Gwandpa01"))
                      (`KismetArrayLibrary.Array_Add` _textarray (make `/Game/Dialog/S_Dialog` "You saw Grandpa?! Where did he go?" "Mama Mush" "/Game/Sounds/Voices/MamaMush/VA_SawGrandpa.VA_SawGrandpa"))
                      (`KismetArrayLibrary.Array_Add` _textarray (make `/Game/Dialog/S_Dialog` "Chop! Chop! Fwah!!!! Fwah!!!! Fiyah!!!!" "Baby Mush" "/Game/Sounds/Voices/BabyMush/VA_BabyNoises.VA_BabyNoises"))
                      (`KismetArrayLibrary.Array_Add` _textarray (make `/Game/Dialog/S_Dialog` "Ooooh…..sounds like Grandpa’s gonna be made into a fine shiitake stir fry. Might wanna get to the kitchen before it’s too late." "Merchant" "/Game/Sounds/Voices/Merchant/VA_Shiitake.VA_Shiitake"))
                      (`KismetArrayLibrary.Array_Add` _textarray (make `/Game/Dialog/S_Dialog` "But how? How do we get to him?" "Mama Mush" "/Game/Sounds/Voices/MamaMush/VA_ButHow.VA_ButHow"))
                      (`KismetArrayLibrary.Array_Add` _textarray (make `/Game/Dialog/S_Dialog` "Last time I saw the key, it was just hangin out on the couch. But…" "Merchant" "/Game/Sounds/Voices/Merchant/VA_TheresAKey.VA_TheresAKey"))
                      (`KismetArrayLibrary.Array_Add` _textarray (make `/Game/Dialog/S_Dialog` "She’s really invested in that game... bet she wouldn’t even notice if you ran right in front of her! We’re gonna need some other kind of distraction…" "Merchant" "/Game/Sounds/Voices/Merchant/VA_InvestedInGame.VA_InvestedInGame"))
                      (set `self.postBabySaved` true)
                      (bind _asshroommate_proto_character (cast `ShroommateProtoCharacter` (`GameplayStatics.GetPlayerCharacter` 0)))
                      (set `ShroommateProtoCharacter.MakeNoiseCheck` true _asshroommate_proto_character)))
                  (else
                    (`KismetArrayLibrary.Array_Add` _textarray (make `/Game/Dialog/S_Dialog` "You might want to think about saving your brother there..." "Merchant" "/Game/Sounds/Voices/Merchant/S_Happy.S_Happy"))))
                (else
                  ;[1 0.09375 0.09375] Kitchen
                  (if (`|EnumEquality` NewParam "NewEnumerator3")
                    (if (`self.grandpaSaved`)
                      (if (`self.postGrandpaSaved`)
                        (`KismetArrayLibrary.Array_Add` _textarray_2 (make `/Game/Dialog/S_Dialog` "There's no way to get on top of that fridge normally. I'm hungry though. Hey, I bet food powers mushrooms up too right?" "Merchant" "/Game/Sounds/Voices/Merchant/VA_NoWayFridge.VA_NoWayFridge"))
                        (else
                          (`KismetArrayLibrary.Array_Add` _textarray_2 (make `/Game/Dialog/S_Dialog` "You're gonna have to find a way to that vent up there above the fridge." "Merchant" "/Game/Sounds/Voices/Merchant/VA_GottaFindVent.VA_GottaFindVent"))
                          (set `self.postGrandpaSaved` true)))
                      (else
                        (`KismetArrayLibrary.Array_Add` _textarray_2 (make `/Game/Dialog/S_Dialog` "Gwandpa!" "Baby Mush" "/Game/Sounds/Voices/BabyMush/VA_Gwandpa02.VA_Gwandpa02"))))
                    (else
                      ;[1 1 1] Attic
                      (if (`|EnumEquality` NewParam "NewEnumerator5")
                        (`KismetArrayLibrary.Array_Add` _textarray_4 (make `/Game/Dialog/S_Dialog` "So you're here, Mushy." "Merchant" "/Game/Sounds/Voices/Merchant/VA_SoYoureHere.VA_SoYoureHere"))
                        (`KismetArrayLibrary.Array_Add` _textarray_4 (make `/Game/Dialog/S_Dialog` "Quite the reunion we got here. Home sweet home, eh?" "Merchant" "/Game/Sounds/Voices/Merchant/VA_QuiteTheReunion.VA_QuiteTheReunion"))
                        (`KismetArrayLibrary.Array_Add` _textarray_4 (make `/Game/Dialog/S_Dialog` "Well..." "Merchant" "/Game/Sounds/Voices/Merchant/VA_Well.VA_Well"))
                        (`KismetArrayLibrary.Array_Add` _textarray_4 (make `/Game/Dialog/S_Dialog` "I must thank ya, my good friend." "Merchant" "/Game/Sounds/Voices/Merchant/VA_MustThankYa.VA_MustThankYa"))
                        (`KismetArrayLibrary.Array_Add` _textarray_4 (make `/Game/Dialog/S_Dialog` "I’ve been looking for a way in here and ya led me right to it. That house deed is mine…!" "Merchant" "/Game/Sounds/Voices/Merchant/VA_HouseDeed.VA_HouseDeed"))
                        (`KismetArrayLibrary.Array_Add` _textarray_4 (make `/Game/Dialog/S_Dialog` "That’s what he was after?!" "Mama Mush" "/Game/Sounds/Voices/MamaMush/VA_WhatHesAfter.VA_WhatHesAfter"))
                        (`KismetArrayLibrary.Array_Add` _textarray_4 (make `/Game/Dialog/S_Dialog` "Indeed. (laughter) I’ve wanted a place for my own for so long…." "Merchant" "/Game/Sounds/Voices/Merchant/VA_WantedOwnPlace.VA_WantedOwnPlace"))
                        (`KismetArrayLibrary.Array_Add` _textarray_4 (make `/Game/Dialog/S_Dialog` "No...you have to stop him, Mushy!" "Grandpa Mush" "/Game/Sounds/Voices/GrandpaMush/VA_StopHimMushy.VA_StopHimMushy"))
                        (set `self.gameEnd` true)))))))))))))

(fn `Teleport`
  (params (location :type "/Game/Dialog/E_CurrentRoom Enum" :default "NewEnumerator0"))
  ;[0.09375 1 0.1357] Garden
  (if (`|EnumEquality` location "NewEnumerator0")
    (`self.K2_TeleportTo` (-14356.0 -25442.0 98.0) (struct :`Yaw` 90.0))
    (set `self.currentRoom` "NewEnumerator0")
    (else
      ;[0.2448 0.499 1] Bathroom
      (if (`|EnumEquality` location "NewEnumerator1")
        (`self.K2_TeleportTo` (-13800.0 -24615.0 100.0))
        (set `self.currentRoom` "NewEnumerator1")
        (else
          ;[1 0.5362 0.09896] Living room
          (if (`|EnumEquality` location "NewEnumerator2")
            (`self.K2_TeleportTo` (-13967.0 -23012.0 202.0) (struct :`Yaw` -180.0))
            (set `self.currentRoom` "NewEnumerator2")
            (else
              ;[1 0.1094 0.1094] Kitchen
              (if (`|EnumEquality` location "NewEnumerator3")
                (`self.K2_TeleportTo` (-12126.0 -23641.0 98.0) (struct :`Yaw` 90.0))
                (set `self.currentRoom` "NewEnumerator3")
                (elif (`|EnumEquality` location "NewEnumerator5")
                  (`self.K2_TeleportTo` (-12762.0 -24481.0 412.0) (struct :`Yaw` 100.0))
                  (set `self.currentRoom` "NewEnumerator5"))))))))))

(fn `UserConstructionScript`)
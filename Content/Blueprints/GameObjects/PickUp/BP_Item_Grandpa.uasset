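; BP_Item_Grandpa is a Grandpa pickup that the player carries after overlapping its box.
; On overlap, if no kitchen item is held, it flags the controller as holding one.
; If the first merchant's GrandpaSaved is false, it then attaches above the player, disables collision, enables input and sets DropGrandCheck on the character.
; While holding an item, the Flatten input squashes the player's Z scale and lowers Grandpa to match, restoring both on release.
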(event `self.Box.OnComponentBeginOverlap`
  (params (OverlappedComponent :type "PrimitiveComponent Object Reference") (OtherActor :type "Actor Object Reference") (OtherComp :type "PrimitiveComponent Object Reference") (OtherBodyIndex :type Integer) (bFromSweep :type Boolean) (SweepResult :type "HitResult Structure (by ref)"))
  (bind _asbp_skill_tree_controller (cast `/Game/Blueprints/BP_SkillTreeController` (`GameplayStatics.GetPlayerController` 0) :!pure true))
  (if (not (`SkillTreeController.haskitchenitem` _asbp_skill_tree_controller))
    (set `SkillTreeController.haskitchenitem` true _asbp_skill_tree_controller)
    (bind _outactors (`GameplayStatics.GetAllActorsOfClass` "/Game/Dialog/BP_Merchant.BP_Merchant_C"))
    (if (not (`/Game/Dialog/BP_Merchant.grandpaSaved` (`|GetArrayItem` _outactors)))
      (`self.K2_AttachToActor` (`GameplayStatics.GetPlayerCharacter` 0) "None" "SnapToTarget" "SnapToTarget" "KeepWorld")
      (`self.K2_AddActorLocalOffset` (0.0 200.0 800.0))
      (`self.SetActorEnableCollision` false)
      (`self.K2_AddActorLocalRotation` (struct))
      (`self.EnableInput` _asbp_skill_tree_controller)
      (bind _asshroommate_proto_character (cast `ShroommateProtoCharacter` (`GameplayStatics.GetPlayerCharacter` 0)))
      (set `ShroommateProtoCharacter.DropGrandCheck` true _asshroommate_proto_character))))

(event `InputAction|Flatten` :consume false
  (params (Key :type "Key Structure"))
  (bind _haskitchenitem (`SkillTreeController.haskitchenitem` (cast `/Game/Blueprints/BP_SkillTreeController` (`GameplayStatics.GetPlayerController` 0) :!pure true)))
  (:`Pressed`
    (if _haskitchenitem
      (`self.SetActorRelativeScale3D` (`GameplayStatics.GetPlayerCharacter` 0) (0.035 0.035 0.02))
      (`self.K2_AddActorLocalOffset` (0.0 0.0 -220.0))))
  (:`Released`
    (if _haskitchenitem
      (`self.SetActorRelativeScale3D` (`GameplayStatics.GetPlayerCharacter` 0) (0.035 0.035 0.035))
      (`self.K2_AddActorLocalOffset` (0.0 0.0 220.0)))))

(fn `UserConstructionScript`)